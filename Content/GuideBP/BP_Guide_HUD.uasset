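; HUD Blueprint that draws the game's score, time and level, plus a game-over screen.
; On BeginPlay it casts the game mode to BP_Guide_GameMode and caches it.
; Each DrawHUD reads that reference and draws colored text at fixed screen positions.
; When the game mode's GameOver flag is set, it also shows GAME OVER and a Press Enter prompt.
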(event EventBeginPlay
  (bind _asbp_guide_game_mode (Utilities|Casting|CastToBP_Guide_GameMode (Game|GetGameMode)))
  (Variables|Default|SetMy_Guide_GameMode _asbp_guide_game_mode))

(event EventDrawHUD
  (params (SizeX :type Integer) (SizeY :type Integer))
  (HUD|DrawText (Utilities|String|BuildString(Integer) "Score: " "" (Variables|/Game/GuideBP/BP_GUIDE_GameMode.BP_Guide_GameMode_C|GetScore (Variables|Default|GetMy_Guide_GameMode))) "(R=1.000000,G=0.773720,B=0.166666,A=1.000000)" 1e+01 1e+01 0 3.0 false)
  (HUD|DrawText (Utilities|String|BuildString(Integer) "Time: " "" (Variables|/Game/GuideBP/BP_GUIDE_GameMode.BP_Guide_GameMode_C|GetTime (Variables|Default|GetMy_Guide_GameMode))) "(R=1.000000,G=0.072917,B=0.072917,A=1.000000)" 3e+02 1e+01 0 3.0 false)
  (HUD|DrawText (Utilities|String|BuildString(Integer) "Level: " "" (Variables|/Game/GuideBP/BP_GUIDE_GameMode.BP_Guide_GameMode_C|GetLevel (Variables|Default|GetMy_Guide_GameMode))) "(R=0.121582,G=0.181696,B=0.864583,A=1.000000)" 5.5e+02 1e+01 0 3.0 false)
  (if (Variables|/Game/GuideBP/BP_GUIDE_GameMode.BP_Guide_GameMode_C|GetGameOver (Variables|Default|GetMy_Guide_GameMode))
    (HUD|DrawText "GAME OVER" "(R=0.515625,G=0.002686,B=0.011058,A=1.000000)" 4e+02 2e+02 0 3.0 false)
    (HUD|DrawText "Press Enter" "(R=0.241882,G=0.864583,B=0.187748,A=1.000000)" 4e+02 4e+02 0 3.0 false)))

(fn ConstructionScript)