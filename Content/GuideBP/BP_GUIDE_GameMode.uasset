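; Game mode for a timed statue-collecting game that tracks score, level, remaining time and game-over state.
; StartGame runs on BeginPlay and RestartGame, resetting state and starting a looping one-second Clock timer.
; Clock counts time down and, at zero, sets GameOver and clears itself.
; StatueCollected adds level-scaled points; every fifth statue grants bonus time and raises the capped level.
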(event Custom|RestartGame
  (Utilities|StartGame))

(event Custom|Clock
  (bind _output_get (Variables|Default|SetTime (- (Variables|Default|GetTime) 1)))
  (if (== _output_get 0)
    (Variables|Default|SetGameOver true)
    (Utilities|Time|ClearTimerbyFunctionName 0 "Clock")))

(event EventBeginPlay
  (Utilities|StartGame))

(fn ConstructionScript)

(fn StatueCollected
  (Variables|Default|SetScore (+ (Variables|Default|GetScore) (* 10 (Variables|Default|GetLevel))))
  (Math|Integer|IncrementInt (Variables|Default|GetStatueCount)
    (:%20%20
      (if (== (Math|Integer|%(Integer) (Variables|Default|GetStatueCount) 5) 0)
        (Variables|Default|SetTime (+ (Variables|Default|GetTime) 15))
        (Variables|Default|SetLevel (Math|Integer|Min(Integer) (+ (Variables|Default|GetLevel) 1) 5))))))